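; First-person player Character Blueprint that handles movement, jumping and camera look through Enhanced Input.
; BeginPlay adds the FPS_IMC mapping context to the local player subsystem.
; Move, Jump and Look actions drive the character, but only strafing is wired, as the forward movement node is disconnected.
; A separate SetGravity function assigns a GravityScale value and is not called within these graphs.
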(event `self.ReceiveBeginPlay`
  ;[1 1 1] Add Input Controls
  (bind _asplayer_controller (cast `PlayerController` (`self.GetController`)))
  (bind _returnvalue (pcsubsystem `EnhancedInputLocalPlayerSubsystem` _asplayer_controller))
  (`/Engine/EditorBlueprintResources/StandardMacros.IsValid` _returnvalue
    (:`Is Valid`
      (`EnhancedInputSubsystemInterface.AddMappingContext` _returnvalue "/Game/Input/FPS_IMC.FPS_IMC" 0 (struct)))))

(event `EnhancedInput|/Game/Input/Move_IA`
  (params (ActionValue :type "Vector2D Structure") (ElapsedSeconds :type "Float (double-precision)") (TriggeredSeconds :type "Float (double-precision)") (InputAction :type "InputAction Object Reference" :default "/Game/Input/Move_IA.Move_IA"))
  ;[1 1 1] Handle Movement
  (:`Triggered`
    (`self.AddMovementInput` (`self.GetActorRightVector`) ActionValue_X)))

(event `EnhancedInput|/Game/Input/Jump_IA`
  (params (ActionValue :type Boolean) (ElapsedSeconds :type "Float (double-precision)") (TriggeredSeconds :type "Float (double-precision)") (InputAction :type "InputAction Object Reference" :default "/Game/Input/Jump_IA.Jump_IA"))
  (:`Triggered`
    (`self.Jump`))
  (:`Completed`
    (`self.StopJumping`)))

(event `EnhancedInput|/Game/Input/Look_IA`
  (params (ActionValue :type "Vector2D Structure") (ElapsedSeconds :type "Float (double-precision)") (TriggeredSeconds :type "Float (double-precision)") (InputAction :type "InputAction Object Reference" :default "/Game/Input/Look_IA.Look_IA"))
  ;[1 1 1] Handle Camera Input
  (:`Triggered`
    (`self.AddControllerYawInput` ActionValue_X)
    (`self.AddControllerPitchInput` ActionValue_Y)))

(fn `Set Gravity`
  (params (`Gravity Scale` :type "Float (single-precision)"))
  (set `self.Gravity Scale` `Gravity Scale`))

(fn `UserConstructionScript`)